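; Default player controller that forwards keyboard, mouse and action input to the possessed BP_DefaultPlayer pawn.
; It caches the pawn as CurrentPlayer on BeginPlay and Possess through a cast, and clears it on UnPossess.
; Movement, look, jump, crouch, run, use and escape-menu inputs become IPossessControl messages on CurrentPlayer, leaving the behavior to the pawn.
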(event `self.ReceiveBeginPlay`
  (`self.InitDefaultPlayer`))

(event `self.ReceivePossess`
  (params (PossessedPawn :type "Pawn Object Reference"))
  (`self.CastPawnToDefaultPlayer` PossessedPawn))

(event `self.ReceiveUnPossess`
  (params (UnpossessedPawn :type "Pawn Object Reference"))
  (set `self.currentPlayer` null) ; Reset Current Player
)

(event `InputAxis|MoveForward`
  (params (AxisValue :type "Float (single-precision)"))
  ;[0 0 0] IPossessControl
  ;;[1 1 1] Movement
  (message `/Game/FleshOfSilence/Misc/Interfaces/IPossesControl.MoveForwardControl` (`self.currentPlayer`) AxisValue))

(event `InputAxis|Turn`
  (params (AxisValue :type "Float (single-precision)"))
  ;[0 0 0] IPossessControl
  ;;[1 1 1] Looking
  (message `/Game/FleshOfSilence/Misc/Interfaces/IPossesControl.TurnControl` (`self.currentPlayer`) AxisValue))

(event `InputAxis|LookUp`
  (params (AxisValue :type "Float (single-precision)"))
  ;[0 0 0] IPossessControl
  ;;[1 1 1] Looking
  (message `/Game/FleshOfSilence/Misc/Interfaces/IPossesControl.LookUpControl` (`self.currentPlayer`) AxisValue))

(event `InputAxis|MoveRight`
  (params (AxisValue :type "Float (single-precision)"))
  ;[0 0 0] IPossessControl
  ;;[1 1 1] Movement
  (message `/Game/FleshOfSilence/Misc/Interfaces/IPossesControl.MoveRightControl` (`self.currentPlayer`) AxisValue))

(event `InputAction|Jump`
  (params (Key :type "Key Structure"))
  (bind _currentplayer (`self.currentPlayer`))
  ;[0 0 0] IPossessControl
  ;;[1 1 1] Jumping
  (:`Pressed`
    (message `/Game/FleshOfSilence/Misc/Interfaces/IPossesControl.JumpControl` _currentplayer))
  (:`Released`
    (message `/Game/FleshOfSilence/Misc/Interfaces/IPossesControl.StopJumpingControl` _currentplayer)))

(event `InputAction|Crouch`
  (params (Key :type "Key Structure"))
  (bind _currentplayer (`self.currentPlayer`))
  ;[0 0 0] IPossessControl
  ;;[1 1 1] Crouch
  (:`Pressed`
    (message `/Game/FleshOfSilence/Misc/Interfaces/IPossesControl.CrouchControl` _currentplayer))
  (:`Released`
    (message `/Game/FleshOfSilence/Misc/Interfaces/IPossesControl.UnCrouchControl` _currentplayer)))

(event `InputAction|Use`
  (params (Key :type "Key Structure"))
  ;[0 0 0] IPossessControl
  ;;[1 1 1] Using
  (:`Pressed`
    (message `/Game/FleshOfSilence/Misc/Interfaces/IPossesControl.UseControl` (`self.currentPlayer`))))

(event `InputAction|Run`
  (params (Key :type "Key Structure"))
  (bind _currentplayer (`self.currentPlayer`))
  ;[0 0 0] IPossessControl
  ;;[1 1 1] Running
  (:`Pressed`
    (message `/Game/FleshOfSilence/Misc/Interfaces/IPossesControl.RunControl` _currentplayer))
  (:`Released`
    (message `/Game/FleshOfSilence/Misc/Interfaces/IPossesControl.StopRunningControl` _currentplayer)))

(event `InputAction|EscapeMenu`
  (params (Key :type "Key Structure"))
  ;[0 0 0] IPossessControl
  ;;[1 1 1] EscapeMenu
  (:`Pressed`
    (message `/Game/FleshOfSilence/Misc/Interfaces/IPossesControl.ToggleEscapeMenuControl` (`self.currentPlayer`))))

(fn `CastPawnToDefaultPlayer`
  (params (pawnObject :type "Pawn Object Reference"))
  (bind _asbp_default_player (cast `/Game/FleshOfSilence/Characters/Player/BP_DefaultPlayer` pawnObject))
  (set `self.currentPlayer` _asbp_default_player))

(fn `InitDefaultPlayer`
  (`self.CastPawnToDefaultPlayer` (`self.K2_GetPawn`)))

(fn `UserConstructionScript`)