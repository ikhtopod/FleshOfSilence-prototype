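; BP_DefaultPlayer is the player character, providing movement, mouse look, jumping, crouching and running.
; It caches the default player controller on possession and BeginPlay, clears it on unpossession, and stores the main game instance.
; ControlGraph exposes custom events for each action, with look scaled by sensitivity and frame time.
; Running temporarily swaps the walk speed, while Use and the pause menu only print placeholder messages.
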(event `self.ReceivePossessed`
  (params (NewController :type "Controller Object Reference"))
  ;[1 1 1] Possessed
  (`self.CastControllerToDefaultPlayerController` NewController))

(event `self.ReceiveUnpossessed`
  (params (OldController :type "Controller Object Reference"))
  ;[1 1 1] Possessed
  (set `self.currentPlayerController` null) ; Reset DefaultPlayerController
)

(event `self.ReceiveBeginPlay`
  (`|ExecutionSequence`
    (:`then_0`
      ;[1 1 1] Possessed
      (`self.InitDefaultPlayerController`))
    (:`then_1`
      (`self.InitMainGameInstance`))))

(event `/Game/FleshOfSilence/Misc/Interfaces/IPossesControl.TurnControl`
  (params (AxisValue :type "Float (single-precision)"))
  ;[0 0 0] PlayerController
  ;;[1 1 1] Looking
  (`self.AddControllerYawInput` (* AxisValue (`self.mouseSensitivity`) (`GameplayStatics.GetWorldDeltaSeconds`))))

(event `/Game/FleshOfSilence/Misc/Interfaces/IPossesControl.MoveForwardControl`
  (params (AxisValue :type "Float (single-precision)"))
  ;[0 0 0] PlayerController
  ;;[1 1 1] Movement
  (`self.AddMovementInput` (`self.GetActorForwardVector`) AxisValue))

(event `/Game/FleshOfSilence/Misc/Interfaces/IPossesControl.MoveRightControl`
  (params (AxisValue :type "Float (single-precision)"))
  ;[0 0 0] PlayerController
  ;;[1 1 1] Movement
  (`self.AddMovementInput` (`self.GetActorRightVector`) AxisValue))

(event `/Game/FleshOfSilence/Misc/Interfaces/IPossesControl.LookUpControl`
  (params (AxisValue :type "Float (single-precision)"))
  ;[0 0 0] PlayerController
  ;;[1 1 1] Looking
  (`self.AddControllerPitchInput` (* AxisValue (`self.mouseSensitivity`) (`GameplayStatics.GetWorldDeltaSeconds`))))

(event `/Game/FleshOfSilence/Misc/Interfaces/IPossesControl.ToggleEscapeMenuControl`
  ;[1 1 1] EscapeMenu with Pausing game
  (`KismetSystemLibrary.PrintString` "Pause Game and Show Menu"))

(event `/Game/FleshOfSilence/Misc/Interfaces/IPossesControl.JumpControl`
  ;[0 0 0] PlayerController
  ;;[1 1 1] Jumping
  (`self.Jump`))

(event `/Game/FleshOfSilence/Misc/Interfaces/IPossesControl.CrouchControl`
  ;[0 0 0] PlayerController
  ;;[1 1 1] Crouch
  (`self.Crouch`))

(event `/Game/FleshOfSilence/Misc/Interfaces/IPossesControl.StopJumpingControl`
  ;[0 0 0] PlayerController
  ;;[1 1 1] Jumping
  (`self.StopJumping`))

(event `/Game/FleshOfSilence/Misc/Interfaces/IPossesControl.UnCrouchControl`
  ;[0 0 0] PlayerController
  ;;[1 1 1] Crouch
  (`self.UnCrouch`))

(event `/Game/FleshOfSilence/Misc/Interfaces/IPossesControl.RunControl`
  (bind _charactermovement (`self.CharacterMovement`))
  ;[0 0 0] PlayerController
  ;;[1 1 1] Running
  (set `self.maxWalkSpeedTmp` (`CharacterMovementComponent.MaxWalkSpeed` _charactermovement))
  (set `CharacterMovementComponent.MaxWalkSpeed` (`self.runningSpeed`) _charactermovement))

(event `/Game/FleshOfSilence/Misc/Interfaces/IPossesControl.StopRunningControl`
  ;[0 0 0] PlayerController
  ;;[1 1 1] Running
  (set `CharacterMovementComponent.MaxWalkSpeed` (`self.maxWalkSpeedTmp`) (`self.CharacterMovement`)))

(event `/Game/FleshOfSilence/Misc/Interfaces/IPossesControl.UseControl`
  ;[0 0 0] PlayerController
  ;;[1 1 1] Using
  (`KismetSystemLibrary.PrintString` "Use!"))

(fn `CastControllerToDefaultPlayerController`
  (params (controllerObject :type "Controller Object Reference"))
  (bind _asbp_default_player_controller (cast `/Game/FleshOfSilence/Characters/Player/BP_DefaultPlayerController` controllerObject))
  (set `self.currentPlayerController` _asbp_default_player_controller))

(fn `InitDefaultPlayerController`
  (`self.CastControllerToDefaultPlayerController` (`GameplayStatics.GetPlayerController` 0)))

(fn `InitMainGameInstance`
  (bind _asmain_game_instance (cast `/Game/FleshOfSilence/Misc/MainGameInstance` (`GameplayStatics.GetGameInstance`)))
  (set `self.mainGameInstance` _asmain_game_instance))

(fn `UserConstructionScript`)